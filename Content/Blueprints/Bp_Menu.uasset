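; Menu actor for a card game, with four clickable buttons that each pick a card count and move limit.
; A click triggers a camera transition, slides the menu from its construction-time transform to a fixed end transform via timeline, and passes both values to the Deck and Logic Blueprints.
; A gate opens shortly afterward, so a later MenuShow event closes it, reverses the slide and transitions the camera back.
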(event OnClicked(Button1)
  (params (TouchedComponent :type Primitive%20Component%20Object%20Reference))
  ;[1 1 1] Menu buttons click logic. Setup number of cards
  (Variables|Default|SetCardNumber 8)
  (Variables|Default|SetMaxMoves 9)
  (Utilities|FlowControl|Sequence
    (:then_0
      ;[1 1 1] Move the menu
      (Default|CallCameraTransition false)
      (bind _position (Timeline|MenuPosition PlayFromStart)
        (:Update
          (Transformation|SetActorTransform (Math|Transform|Lerp(Transform) (Variables|Default|GetStartTransform) (Variables|Default|GetEndTransform) _position)))))
    (:then_1
      ;[1 1 1] Set variables to other bps
      (Default|SetCardNumber (Variables|GameControl|GetDeck) (Variables|Default|GetCardNumber) (Variables|Default|GetMaxMoves))
      (Default|SetCardNumber (Variables|GameControl|GetLogic) (Variables|Default|GetCardNumber) (Variables|Default|GetMaxMoves)))
    (:then_2
      (Utilities|FlowControl|Delay 0.1)
      (Utilities|FlowControl|Gate true) ; enters at Open
    )))

(event OnClicked(Button4)
  (params (TouchedComponent :type Primitive%20Component%20Object%20Reference))
  ;[1 1 1] Menu buttons click logic. Setup number of cards
  (Variables|Default|SetCardNumber 20)
  (Variables|Default|SetMaxMoves 27)
  (Utilities|FlowControl|Sequence
    (:then_0
      ;[1 1 1] Move the menu
      (Default|CallCameraTransition false)
      (bind _position (Timeline|MenuPosition PlayFromStart)
        (:Update
          (Transformation|SetActorTransform (Math|Transform|Lerp(Transform) (Variables|Default|GetStartTransform) (Variables|Default|GetEndTransform) _position)))))
    (:then_1
      ;[1 1 1] Set variables to other bps
      (Default|SetCardNumber (Variables|GameControl|GetDeck) (Variables|Default|GetCardNumber) (Variables|Default|GetMaxMoves))
      (Default|SetCardNumber (Variables|GameControl|GetLogic) (Variables|Default|GetCardNumber) (Variables|Default|GetMaxMoves)))
    (:then_2
      (Utilities|FlowControl|Delay 0.1)
      (Utilities|FlowControl|Gate true) ; enters at Open
    )))

(event OnClicked(Button2)
  (params (TouchedComponent :type Primitive%20Component%20Object%20Reference))
  ;[1 1 1] Menu buttons click logic. Setup number of cards
  (Variables|Default|SetCardNumber 12)
  (Variables|Default|SetMaxMoves 14)
  (Utilities|FlowControl|Sequence
    (:then_0
      ;[1 1 1] Move the menu
      (Default|CallCameraTransition false)
      (bind _position (Timeline|MenuPosition PlayFromStart)
        (:Update
          (Transformation|SetActorTransform (Math|Transform|Lerp(Transform) (Variables|Default|GetStartTransform) (Variables|Default|GetEndTransform) _position)))))
    (:then_1
      ;[1 1 1] Set variables to other bps
      (Default|SetCardNumber (Variables|GameControl|GetDeck) (Variables|Default|GetCardNumber) (Variables|Default|GetMaxMoves))
      (Default|SetCardNumber (Variables|GameControl|GetLogic) (Variables|Default|GetCardNumber) (Variables|Default|GetMaxMoves)))
    (:then_2
      (Utilities|FlowControl|Delay 0.1)
      (Utilities|FlowControl|Gate true) ; enters at Open
    )))

(event OnClicked(Button3)
  (params (TouchedComponent :type Primitive%20Component%20Object%20Reference))
  ;[1 1 1] Menu buttons click logic. Setup number of cards
  (Variables|Default|SetCardNumber 16)
  (Variables|Default|SetMaxMoves 20)
  (Utilities|FlowControl|Sequence
    (:then_0
      ;[1 1 1] Move the menu
      (Default|CallCameraTransition false)
      (bind _position (Timeline|MenuPosition PlayFromStart)
        (:Update
          (Transformation|SetActorTransform (Math|Transform|Lerp(Transform) (Variables|Default|GetStartTransform) (Variables|Default|GetEndTransform) _position)))))
    (:then_1
      ;[1 1 1] Set variables to other bps
      (Default|SetCardNumber (Variables|GameControl|GetDeck) (Variables|Default|GetCardNumber) (Variables|Default|GetMaxMoves))
      (Default|SetCardNumber (Variables|GameControl|GetLogic) (Variables|Default|GetCardNumber) (Variables|Default|GetMaxMoves)))
    (:then_2
      (Utilities|FlowControl|Delay 0.1)
      (Utilities|FlowControl|Gate true) ; enters at Open
    )))

(event Custom|MenuShow
  (Utilities|FlowControl|Gate true :!label _label
    (:Exit
      (Utilities|FlowControl|Sequence
        (:then_0
          (goto _label Close))
        (:then_1
          ;[1 1 1] Move the menu
          (Default|CallCameraTransition true)
          (bind _position (Timeline|MenuPosition Reverse)
            (:Update
              (Transformation|SetActorTransform (Math|Transform|Lerp(Transform) (Variables|Default|GetStartTransform) (Variables|Default|GetEndTransform) _position)))))))))

(event EventBeginPlay)

(event EventActorBeginOverlap
  (params (OtherActor :type Actor%20Object%20Reference)))

(event EventTick
  (params (DeltaSeconds :type Float%20%28single-precision%29)))

(fn ConstructionScript
  (Variables|Default|SetStartTransform (Transformation|GetActorTransform))
  (Variables|Default|SetEndTransform (Math|Transform|MakeTransform "-1100.000000,622.000000,447.000000" "0,-180.000000, 0")))